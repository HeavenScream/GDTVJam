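; Poison hazard area with a sphere trigger that applies poison to the third-person character through the Gameplay Ability System.
; On overlap it repeatedly activates the poison ability on the character's ability system component, looping each second through a retriggerable delay while a single inside flag holds.
; Leaving clears that flag and removes effects tagged as poison area.
; The construction script sizes the sphere from the area radius variable.
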(event OnComponentBeginOverlap(Sphere)
  (params (OverlappedComponent :type Primitive%20Component%20Object%20Reference) (OtherActor :type Actor%20Object%20Reference) (OtherComp :type Primitive%20Component%20Object%20Reference) (OtherBodyIndex :type Integer) (bFromSweep :type Boolean) (SweepResult :type Hit%20Result%20Structure%20%28by%20ref%29))
  (bind _output_get (Variables|Default|SetStepedIn true))
  (bind _asbp_third_person_character (Utilities|Casting|CastToBP_ThirdPersonCharacter OtherActor))
  (if _output_get :!label _label
    (Abilities|TryActivateAbilitybyClass (Variables|/Game/ThirdPerson/Blueprints/BP_ThirdPersonCharacter.BP_ThirdPersonCharacter_C|GetBP_AbilitySystemComponent _asbp_third_person_character) "/Game/GAS/BP_GAB_PoisonPlayer.BP_GAB_PoisonPlayer_C" true)
    (Utilities|FlowControl|RetriggerableDelay 1.0)
    (goto _label)))

(event OnComponentEndOverlap(Sphere)
  (params (OverlappedComponent :type Primitive%20Component%20Object%20Reference) (OtherActor :type Actor%20Object%20Reference) (OtherComp :type Primitive%20Component%20Object%20Reference) (OtherBodyIndex :type Integer))
  (Variables|Default|SetStepedIn false)
  (bind _asbp_third_person_character (Utilities|Casting|CastToBP_ThirdPersonCharacter OtherActor))
  (GameplayEffects|RemoveActiveEffectswithTags (Variables|/Game/ThirdPerson/Blueprints/BP_ThirdPersonCharacter.BP_ThirdPersonCharacter_C|GetBP_AbilitySystemComponent _asbp_third_person_character) "(GameplayTags=((TagName=\"Ability.PoisonArea\")))")
  (GameplayEffects|RemoveActiveGameplayEffect :self (Variables|/Game/ThirdPerson/Blueprints/BP_ThirdPersonCharacter.BP_ThirdPersonCharacter_C|GetBP_AbilitySystemComponent _asbp_third_person_character)))

(event EventBeginPlay)

(event Collision|EventActorBeginOverlap
  (params (OtherActor :type Actor%20Object%20Reference)))

(event EventTick
  (params (DeltaSeconds :type Float%20%28single-precision%29)))

(fn ConstructionScript
  (Components|Sphere|SetSphereRadius (Variables|Default|GetSphere) (Variables|Default|GetAreaRadius) true))