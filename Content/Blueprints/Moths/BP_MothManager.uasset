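; Moth area manager that populates its SpawnArea with dead moths and turns them into toxic ones while the player is inside.
; Shortly after BeginPlay, it rolls SpawnChance at each overlapping spawn-location actor, spawning and tracking a dead moth or destroying the marker.
; A randomized timer replaces a random dead moth with a toxic one, re-rolling its interval each time, until the player leaves or none remain.
; OnCollectedMoth destroys and untracks collected moths.
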(event OnComponentBeginOverlap(SpawnArea)
  (params (OverlappedComponent :type Primitive%20Component%20Object%20Reference) (OtherActor :type Actor%20Object%20Reference) (OtherComp :type Primitive%20Component%20Object%20Reference) (OtherBodyIndex :type Integer) (bFromSweep :type Boolean) (SweepResult :type Hit%20Result%20Structure%20%28by%20ref%29))
  (Utilities|Casting|CastToBP_ThirdPersonCharacter OtherActor)
  (CallFunction|StartMothTimer))

(event OnComponentEndOverlap(SpawnArea)
  (params (OverlappedComponent :type Primitive%20Component%20Object%20Reference) (OtherActor :type Actor%20Object%20Reference) (OtherComp :type Primitive%20Component%20Object%20Reference) (OtherBodyIndex :type Integer))
  (Utilities|Casting|CastToBP_ThirdPersonCharacter OtherActor)
  (Utilities|Time|ClearandInvalidateTimerbyHandle (Variables|Default|GetTimerHandle)))

(event Custom|Spawn%20random%20moth%20shit
  (bind _deadmotharray (Variables|Default|GetDeadMothArray))
  (if (== (Utilities|Array|Length (Variables|Default|GetDeadMothArray)) 0)
    (Utilities|Time|ClearandInvalidateTimerbyHandle (Variables|Default|GetTimerHandle))
    (else
      (Variables|Default|SetSpawnMothIndex (Math|Random|RandomInteger (Utilities|Array|Length (Variables|Default|GetDeadMothArray))))
      (CallFunction|SpawnToxicMoth)
      (Actor|DestroyActor (Utilities|Array|Get(acopy) _deadmotharray (Variables|Default|GetSpawnMothIndex)))
      (Utilities|Array|RemoveIndex _deadmotharray (Variables|Default|GetSpawnMothIndex))
      (CallFunction|StartMothTimer))))

(event Custom|StartMothTimer
  (bind _returnvalue (Utilities|Time|SetTimerbyEvent (delegate Custom|Spawn%20random%20moth%20shit) (Math|Random|RandomFloatinRange 3.0 6.5) true))
  (Variables|Default|SetTimerHandle _returnvalue))

(event EventBeginPlay
  (Utilities|FlowControl|Delay 1.0)
  (Variables|Default|SetOverlapping%20Actors (Collision|GetOverlappingActors (Variables|Default|GetSpawnArea) "/Game/Blueprints/Moths/BP_MothSpawnLocation.BP_MothSpawnLocation_C" :!class /Script/Engine.PrimitiveComponent))
  (for _array_element (Variables|Default|GetOverlapping%20Actors)
    (if (CallFunction|ShouldSpawnMoth)
      (CallFunction|SpawnDeadMoth _array_element)
      (else
        (Actor|DestroyActor _array_element))))
  (if (Utilities|Array|IsEmpty (Variables|Default|GetOverlapping%20Actors))
    (Development|PrintString "Actor manager didnt spawn any moths")))

(fn ConstructionScript)

(fn SpawnDeadMoth
  (params (SpawnActor :type Actor%20Object%20Reference))
  (bind _returnvalue (Game|SpawnActorfromClass "/Game/Blueprints/Moths/BP_DeadMoth.BP_DeadMoth_C" (Transformation|GetActorTransform SpawnActor) "AlwaysSpawn" "MultiplyWithRoot" 0 0))
  (Utilities|Array|Add (Variables|Default|GetDeadMothArray) _returnvalue)
  (Default|OnMothSpawned _returnvalue self))

(fn ShouldSpawnMoth
  (return (< (Math|Random|RandomIntegerinRange 0 100) (Variables|Default|GetSpawnChance))))

(fn SpawnToxicMoth
  (Game|SpawnActorfromClass "/Game/AI/BP_Motherfucka.BP_Motherfucka_C" (CallFunction|GetTransformfromActorforSpawning (Utilities|Array|Get(acopy) (Variables|Default|GetDeadMothArray) (Variables|Default|GetSpawnMothIndex))) "Undefined" "MultiplyWithRoot" 0 0))

(fn OnCollectedMoth
  (params (CollectedMoth :type BP%20Dead%20Moth%20Object%20Reference))
  (LocalVariables|SetCollectedMothIndex (Utilities|Array|FindItem (Variables|Default|GetDeadMothArray) CollectedMoth))
  (Actor|DestroyActor (Utilities|Array|Get(acopy) (Variables|Default|GetDeadMothArray) (LocalVariables|GetCollectedMothIndex)))
  (Utilities|Array|RemoveIndex (Variables|Default|GetDeadMothArray) (LocalVariables|GetCollectedMothIndex)))

(fn GetTransformfromActorforSpawning
  (params (self2 :type Actor%20Object%20Reference))
  (bind _returnvalue (Transformation|GetActorTransform self2))
  (bind (_location _rotation _scale) (Math|Transform|BreakTransform _returnvalue))
  (bind (_x _y _z) (Math|Vector|BreakVector _location))
  (return (Math|Transform|MakeTransform (Math|Vector|MakeVector _x _y (+ _z 5e+01)) _rotation _scale)))