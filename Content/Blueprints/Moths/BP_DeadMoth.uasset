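; BP_DeadMoth is a collectible dead moth that feeds the player's Souls attribute and is tracked by a moth manager.
; On BeginPlay it picks a random pose mesh and yaw.
; Player character overlap with its box or a DamageAI event triggers collection, calling SetSouls on BP_Attributes and playing sound and effects.
; It then notifies the MothManager, stored through OnMothSpawned, without destroying itself.
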(event OnComponentBeginOverlap(Box)
  (params (OverlappedComponent :type Primitive%20Component%20Object%20Reference) (OtherActor :type Actor%20Object%20Reference) (OtherComp :type Primitive%20Component%20Object%20Reference) (OtherBodyIndex :type Integer) (bFromSweep :type Boolean) (SweepResult :type Hit%20Result%20Structure%20%28by%20ref%29))
  (Utilities|Casting|CastToBP_ThirdPersonCharacter OtherActor)
  (CallFunction|OnCollectedThisMoth))

(event EventBeginPlay
  (Components|StaticMesh|SetStaticMesh (Variables|Default|GetDeadMoth) (.OutItem (Utilities|Array|Random (Variables|Default|GetDeadMothPoses))))
  (Transformation|SetRelativeRotation (Variables|Default|GetDeadMoth) (Math|Rotator|MakeRotator 9e+01 0.0 (Math|Random|RandomFloatinRange 0.0 3.6e+02)) false false))

(event Collision|EventActorBeginOverlap
  (params (OtherActor :type Actor%20Object%20Reference)))

(event EventTick
  (params (DeltaSeconds :type Float%20%28single-precision%29)))

(event EventDamageAI
  (CallFunction|OnCollectedThisMoth))

(fn ConstructionScript)

(fn OnMothSpawned
  (params (MothManager :type BP%20Moth%20Manager%20Object%20Reference))
  (Variables|Default|SetMothManager MothManager))

(fn OnCollectedThisMoth
  (bind _returnvalue (Game|Player|GetPlayerPawn 0))
  (Default|SetSouls (Actor|GetComponentbyClass _returnvalue "/Game/ThirdPerson/Blueprints/BP_Attributes.BP_Attributes_C") 1)
  (Audio|PlaySound2D (Variables|Default|GetOnCollected_SFX) 1.0 1.0 0.0 0 _returnvalue)
  (Niagara|SpawnSystematLocation (Variables|Default|GetOnCollected_FX) (+ (Transformation|GetActorLocation) "0.000000,0.000000,50.000000"))
  (Default|OnCollectedMoth (Variables|Default|GetMothManager) self))