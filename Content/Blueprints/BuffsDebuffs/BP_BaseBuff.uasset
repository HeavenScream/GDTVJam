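; Base pickup actor for buffs and debuffs, with an empty OnPickedUp hook that receives the collecting player character.
; When a BP_ThirdPersonCharacter overlaps its box, it disables that collision, hides itself, plays collection VFX and sound, then calls OnPickedUp.
; A DamageAI event also calls OnPickedUp on the first player's pawn and hides the actor, skipping the effects and leaving collision untouched.
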(event OnComponentBeginOverlap(Box)
  (params (OverlappedComponent :type Primitive%20Component%20Object%20Reference) (OtherActor :type Actor%20Object%20Reference) (OtherComp :type Primitive%20Component%20Object%20Reference) (OtherBodyIndex :type Integer) (bFromSweep :type Boolean) (SweepResult :type Hit%20Result%20Structure%20%28by%20ref%29))
  (bind _asbp_third_person_character (Utilities|Casting|CastToBP_ThirdPersonCharacter OtherActor))
  (bind _output_get (Variables|Default|SetAs%20BP%20Third%20Person%20Character _asbp_third_person_character))
  (Collision|SetCollisionEnabled (Variables|Default|GetBox) "NoCollision")
  (Rendering|SetActorHiddenInGame true)
  (Niagara|SpawnSystematLocation (Variables|Default|GetOnCollected_FX) (+ (Transformation|GetActorLocation) "0.000000,0.000000,50.000000"))
  (Audio|PlaySound2D (Variables|Default|GetOnCollected_SFX) 1.0 1.0 0.0 0 0)
  (Buffs|OnPickedUp _output_get))

(event OnComponentEndOverlap(Box)
  (params (OverlappedComponent :type Primitive%20Component%20Object%20Reference) (OtherActor :type Actor%20Object%20Reference) (OtherComp :type Primitive%20Component%20Object%20Reference) (OtherBodyIndex :type Integer)))

(event EventBeginPlay)

(event EventDamageAI
  (bind _asbp_third_person_character (Utilities|Casting|CastToBP_ThirdPersonCharacter (Game|Player|GetPlayerPawn 0)))
  (Buffs|OnPickedUp _asbp_third_person_character)
  (Rendering|SetActorHiddenInGame true))

(fn ConstructionScript)

(fn OnPickedUp
  (params (Instigator :type BP%20Third%20Person%20Character%20Object%20Reference)))