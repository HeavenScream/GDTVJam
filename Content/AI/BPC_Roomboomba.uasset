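; AI controller for the Roomboomba bot, apparently built on an inherited Moth behavior of wandering, pursuit and explosion.
; On possess it calls StartEscape and starts a looping timer for Vacuuming.
; Vacuuming applies radial damage ahead of and below the pawn, drawing a debug sphere each tick.
; The Explosion event is empty here, and the other Moth calls and variable setters sit unconnected.
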(event Custom|Vacuuming
  (bind _returnvalue (Pawn|GetControlledPawn))
  (bind _radius (Variables|Default|GetRadius))
  (bind _returnvalue_2 (Transformation|GetActorForwardVector _returnvalue))
  (bind _returnvalue_3 (Transformation|GetActorLocation _returnvalue))
  (bind _returnvalue_4 (* _returnvalue_2 4e+02))
  (bind _returnvalue_5 (+ _returnvalue_3 _returnvalue_4))
  (bind _returnvalue_6 (- _returnvalue_5 "0.000000,0.000000,200.000000"))
  ;[0.15 0.15 0.15 0.5] Apply Damage
  (Game|Damage|ApplyRadialDamage (Variables|Default|GetDamage) _returnvalue_6 _radius 0 0 _returnvalue self false "ECC_WorldStatic")
  ;[0.15 0.15 0.15 0.5] Debug
  (Rendering|Debug|DrawDebugSphere _returnvalue_6 _radius 12 "(R=1.000000,G=1.000000,B=1.000000,A=1.000000)" 0.2 1.0))

(event EventExplosion
  ;[0.15 0.15 0.15 0.5] Moth
)

(event EventPossess
  (params (PossessedPawn :type Pawn%20Object%20Reference))
  ;[0.15 0.15 0.15 0.5] The bot waits 3 seconds, after which it starts running forward, turning when it encounters an obstacle. Also, every 3 seconds, with a 10% chance, the bot can start chasing the player. If the pursuit begins, a 10-second timer is activated, after which the 'Explosion' function will be called. The 'Explosion' function will also be called if the bot catches up with the player. This description is true if all variables in the Moth categories have standard values.
  (Class|RombaController|StartEscape)
  (Utilities|Time|SetTimerbyFunctionName 0 "Vacuuming" 0.1 true))

(fn ConstructionScript)