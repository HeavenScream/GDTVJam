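; Moth AI component with dormant, pursuit, escape and explosion behaviors, apparently still work in progress.
; On possession it calls a recurring pursuit attempt and a pre-explosion timer, whose bodies are not in this graph.
; Explosion prints a debug message and destroys the referenced actor, while Tick prints the escape, pursuit and dormant flags on screen.
; Unconnected nodes lay out the state, movement, turning and explosion functions and tuning variables without running.
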(event EventExplosion
  (Development|PrintString "Boom, destroy")
  (Actor|DestroyActor (Variables|Default|Getref)))

(event EventTick
  (params (DeltaSeconds :type Float%20%28single-precision%29))
  (Development|PrintString (Utilities|String|ToString(Boolean) (Variables|Default|GetbIsEscape)) true false "(R=0.138690,G=1.000000,B=0.000000,A=1.000000)" 0.0)
  (Development|PrintString (Utilities|String|ToString(Boolean) (Variables|Default|GetbIsPursuit)) true false "(R=0.000000,G=0.004941,B=1.000000,A=1.000000)" 0.0)
  (Development|PrintString (Utilities|String|ToString(Boolean) (Variables|Default|GetbIsDormant)) true false "(R=1.000000,G=0.114046,B=0.000000,A=1.000000)" 0.0))

(event EventPossess
  (params (PossessedPawn :type Pawn%20Object%20Reference))
  (Class|RombaController|ConstantAttemptPursuit)
  (Class|RombaController|ActivateTimerBeforeExplosion))

(fn ConstructionScript)