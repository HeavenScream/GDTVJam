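; AI controller for a moth that wanders, then homes in on the player and destroys itself on arrival, printing "Boom".
; On possess it adds a sideways sensor capsule to the character and drives it forward on a fast looping timer.
; Capsule overlaps, ignoring pawns and dynamic objects, trigger random yaw turns, retried after a delay while still overlapping.
; A randomly timed Pursuit starts AIMoveTo toward the player and stops the wander timer.
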(event Custom|On%20Begin%20Overlap
  (params (OverlappedComponent :type Primitive%20Component%20Object%20Reference) (OtherActor :type Actor%20Object%20Reference) (OtherComp :type Primitive%20Component%20Object%20Reference) (OtherBodyIndex :type Integer) (bFromSweep :type Boolean) (SweepResult :type Hit%20Result%20Structure%20%28by%20ref%29))
  (|TurningAfteraCollision (stale EventPossess PossessedPawn) (stale EventPossess _capsule_collision)))

(event Custom|Escape
  (Pawn|Input|AddMovementInput (stale EventPossess PossessedPawn) (Transformation|GetActorForwardVector (stale EventPossess PossessedPawn)) 1.0 false))

(event Custom|Pursuit
  (AI|AIMoveTo (stale EventPossess PossessedPawn) "0, 0, 0" (Game|Player|GetPlayerPawn 0) 5.0 false
    (:then
      (CallFunction|StoptEscape))
    (:OnSuccess
      (Development|PrintString "Boom" true false "(R=0.000000,G=0.660000,B=1.000000,A=1.000000)" 5.0)
      (Actor|DestroyActor (stale EventPossess PossessedPawn)))))

(event Custom|Stopt%20Escape
  (Utilities|Time|ClearandInvalidateTimerbyHandle (stale EventPossess _returnvalue)))

(event EventPossess
  (params (PossessedPawn :type Pawn%20Object%20Reference))
  (bind _capsule_collision (|CreationAndSetupCapsuleCollision PossessedPawn "30.000000,0.000000,0.000000" 3e+01 3e+01))
  (Collision|BindEventtoOnComponentBeginOverlap _capsule_collision (delegate Custom|On%20Begin%20Overlap))
  (bind _returnvalue (Utilities|Time|SetTimerbyEvent (delegate Custom|Escape) 0.02 true))
  (Utilities|Time|SetTimerbyEvent (delegate Custom|Pursuit) (Math|Random|RandomFloatinRange 1e+01 3e+01)))

(event EventEndPlay
  (params (EndPlayReason :type EEndPlayReason%20Enum :default "Destroyed"))
  (CallFunction|StoptEscape))

(fn ConstructionScript)