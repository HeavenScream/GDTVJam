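; AI controller for a Roomba-style "moth" enemy that turns away on collisions and can charge the player, then explode.
; On possess it adds a forward capsule whose overlaps trigger random yaw turns; the looping Escape timer is empty, with forward movement unwired.
; A randomly delayed pursuit timer rolls attack chance, optionally requiring this moth be nearest the player, then checks range.
; Pursuit starts a fuse; explosion only prints and destroys the pawn.
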(event Custom|On%20Begin%20Overlap
  (params (OverlappedComponent :type Primitive%20Component%20Object%20Reference) (OtherActor :type Actor%20Object%20Reference) (OtherComp :type Primitive%20Component%20Object%20Reference) (OtherBodyIndex :type Integer) (bFromSweep :type Boolean) (SweepResult :type Hit%20Result%20Structure%20%28by%20ref%29))
  (Development|PrintString (Utilities|GetDisplayName OtherActor))
  (|TurningAfteraCollision (Pawn|GetControlledPawn) (stale EventPossess _capsule_collision)))

(event Custom|Escape)

(event Custom|Explosion
  (Development|PrintString "Boom" true false "(R=0.000000,G=0.660000,B=1.000000,A=1.000000)" 5.0)
  (Actor|DestroyActor (Pawn|GetControlledPawn)))

(event Custom|Pursuit
  (bind _maximum_detection_distance (Variables|Pursuit|GetMaximum%20Detection%20Distance))
  (if (Math|Random|RandomBoolwithWeight (/ (Variables|Pursuit|GetAttack%20chance) 1e+02))
    (if (Variables|Pursuit|GetProximity%20check?)
      (bind _moths (Utilities|GetAllMoths))
      (if (== (AI|GetAIController (.ReturnValue (Actor|FindNearestActor (Transformation|GetActorLocation (Game|Player|GetPlayerPawn 0)) _moths))) self)
        (if (or (<= (Transformation|GetDistanceTo (Game|Player|GetPlayerPawn 0) (Pawn|GetControlledPawn)) _maximum_detection_distance) (== _maximum_detection_distance 0.0)) :!label _label
          (if (Variables|Pursuit|GetPursuit?)
            (AI|AIMoveTo (Pawn|GetControlledPawn) "0, 0, 0" (Game|Player|GetPlayerPawn 0) 5.0 false
              (:then
                (CallFunction|ActivationExplosion)
                (Variables|Pursuit|SetPursuit? false)
                (Utilities|Array|Clear (Variables|Actor|GetTags)))
              (:OnSuccess
                (CallFunction|Explosion))))))
      (else
        (goto _label)))))

(event Custom|Activation%20Pursuit
  (if (Variables|Pursuit|GetWill%20there%20be%20persecution?)
    (Utilities|Time|SetTimerbyEvent (delegate Custom|Pursuit) (Math|Random|RandomFloatinRange (Variables|Pursuit|GetMinimum%20delay%20before%20pursuit%20begins) (Variables|Pursuit|GetMaximum%20delay%20before%20pursuit%20begins)) (Variables|Pursuit|GetProximity%20check?))))

(event Custom|Activation%20Explosion
  (Utilities|Time|ClearTimerbyFunctionName 0 "Escape")
  (Utilities|Time|SetTimerbyEvent (delegate Custom|Explosion) (Variables|Pursuit|GetTime%20before%20explosion)))

(event EventUnPossess
  (params (UnpossessedPawn :type Pawn%20Object%20Reference))
  (Utilities|Time|ClearTimerbyFunctionName 0 "Escape")
  (Utilities|Time|ClearTimerbyFunctionName 0 "Pursuit")
  (Actor|DestroyActor))

(event EventPossess
  (params (PossessedPawn :type Pawn%20Object%20Reference))
  (bind _capsule_collision (|CreationAndSetupCapsuleCollision PossessedPawn (Variables|Capsule|GetRelative%20Capsule%20Location) (Variables|Capsule|GetRadius%20Casule) (Variables|Capsule|GetHalf%20Height%20Casule)))
  (Collision|BindEventtoOnComponentBeginOverlap _capsule_collision (delegate Custom|On%20Begin%20Overlap))
  (Utilities|Time|SetTimerbyEvent (delegate Custom|Escape) 0.02 true)
  (CallFunction|ActivationPursuit))

(fn ConstructionScript)