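; BP_Test is a test actor that exercises gameplay abilities, including a lantern shine that damages what it touches.
; On BeginPlay it grants a list of ability classes and activates BP_Intoxified, while debug keys trigger BP_Dash and BP_Shine.
; ActivateShine and DeactivateShine events toggle the lantern's intensity and the sphere's radius and collision.
; Actors that begin overlapping the sphere receive a DamageAI message.
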(event OnComponentBeginOverlap(Sphere)
  (params (OverlappedComponent :type Primitive%20Component%20Object%20Reference) (OtherActor :type Actor%20Object%20Reference) (OtherComp :type Primitive%20Component%20Object%20Reference) (OtherBodyIndex :type Integer) (bFromSweep :type Boolean) (SweepResult :type Hit%20Result%20Structure%20%28by%20ref%29))
  (Class|BPIPlayerInteractsWorld|DamageAI(Message) OtherActor))

(event EventBeginPlay
  (for _array_element (Variables|Default|GetAbility%20Class)
    (GameplayAbilities|GiveAbility (Variables|Default|GetBP_AbilitySystemComponent) _array_element 0 -1))
  (Abilities|TryActivateAbilitybyClass (Variables|Default|GetBP_AbilitySystemComponent) "/Game/GAS/BP_Intoxified.BP_Intoxified_C" true))

(event Collision|EventActorBeginOverlap
  (params (OtherActor :type Actor%20Object%20Reference)))

(event EventTick
  (params (DeltaSeconds :type Float%20%28single-precision%29)))

(event EventActivateShine
  (bind _sphere (Variables|Default|GetSphere))
  ;[0.15 0.15 0.15 0.5] ShineOn
  (Rendering|Components|Light|SetIntensity (Variables|Default|GetLanternlight) 5e+03)
  (Components|Sphere|SetSphereRadius _sphere 5e+02 true)
  (Collision|SetCollisionEnabled _sphere "QueryOnly"))

(event EventDeactivateShine
  (bind _sphere (Variables|Default|GetSphere))
  ;[0.15 0.15 0.15 0.5] ShineOn
  (Rendering|Components|Light|SetIntensity (Variables|Default|GetLanternlight) 0.0)
  (Collision|SetCollisionEnabled _sphere "NoCollision")
  (Components|Sphere|SetSphereRadius _sphere 32.0 true))

(event Input|KeyboardEvents|DebugKey2
  (params (Key :type Key%20Structure :default "None") (ActionValue :type Input%20Action%20Value%20Structure))
  ;[0.15 0.15 0.15 0.5] Skills
  (:Pressed
    (Abilities|TryActivateAbilitybyClass (Variables|Default|GetBP_AbilitySystemComponent) "/Game/GAS/BP_Shine.BP_Shine_C" true)))

(event Input|KeyboardEvents|DebugKey1
  (params (Key :type Key%20Structure :default "None") (ActionValue :type Input%20Action%20Value%20Structure))
  ;[0.15 0.15 0.15 0.5] Skills
  (:Pressed
    (Abilities|TryActivateAbilitybyClass (Variables|Default|GetBP_AbilitySystemComponent) "/Game/GAS/BP_Dash.BP_Dash_C" true)))

(fn ConstructionScript)