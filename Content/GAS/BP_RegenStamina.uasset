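; Gameplay Ability that regenerates the avatar's stamina in periodic steps after attribute changes.
; On activation it commits, caches max values from BP_Attributes and binds to its attribute-change event.
; Changes start a looping one-second timer unless regeneration is running below max; each tick passes a negative amount to SetStamina, clearing the timer near max.
; EndAbility is never reached, so the ability stays active as a listener.
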(event Custom|OnAttributesChanged
  (params (Health :type Float%20%28double-precision%29) (Stamina :type Float%20%28double-precision%29))
  (if (not (and (Variables|Default|GetAlreadyRegenerating) (< Stamina (Variables|Default|GetMax%20Stamina))))
    (Variables|Default|SetAlreadyRegenerating true)
    (bind _returnvalue (Utilities|Time|SetTimerbyEvent (delegate Custom|StartRegen) 1.0 true))
    (Variables|Default|SetTimerHandle _returnvalue)))

(event Custom|StartRegen
  (if (>= (+ (Variables|/Game/ThirdPerson/Blueprints/BP_Attributes.BP_Attributes_C|GetStamina (Variables|Default|GetAttributes)) 4.0) (Variables|Default|GetMax%20Stamina))
    (Utilities|Time|ClearandInvalidateTimerbyHandle (Variables|Default|GetTimerHandle))
    (Variables|Default|SetAlreadyRegenerating false))
  (Default|SetStamina (Variables|Default|GetAttributes) -4.0))

(event Ability|EventActivateAbility
  (Ability|CommitAbility)
  (Variables|Default|SetAttributes (Actor|GetComponentbyClass (Ability|GetAvatarActorfromActorInfo) "/Game/ThirdPerson/Blueprints/BP_Attributes.BP_Attributes_C"))
  (bind (_maxhealth _maxstamina) (Default|GetAttributesMax (Variables|Default|GetAttributes)))
  (Variables|Default|SetMax%20Health _maxhealth)
  (Variables|Default|SetMax%20Stamina _maxstamina)
  (EventDispatchers|BindEventtoOnAttributesChanged (Variables|Default|GetAttributes) (delegate Custom|OnAttributesChanged)))

(event Ability|EventOnEndAbility
  (params (bWasCancelled :type Boolean)))