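; BP_Fly is a Gameplay Ability that launches the third-person character upward with its wings out.
; It commits, checks BP_Attributes Stamina against RequiredStamina, then activates the wings and passes that amount to SetStamina.
; A dash-up montage plays alongside a constant root-motion force along the actor's up vector.
; Montage completion or interruption deactivates the wings and ends the ability; a failed check or cast just ends it.
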(event Ability|EventActivateAbility
  (bind _returnvalue (Ability|GetAvatarActorfromActorInfo))
  (bind _returnvalue_2 (Ability|GetAvatarActorfromActorInfo))
  (bind _returnvalue_3 (Actor|GetComponentbyClass _returnvalue_2 "/Game/ThirdPerson/Blueprints/BP_Attributes.BP_Attributes_C"))
  (Ability|CommitAbility)
  (if (>= (Variables|/Game/ThirdPerson/Blueprints/BP_Attributes.BP_Attributes_C|GetStamina _returnvalue_3) (Variables|Default|GetRequiredStamina))
    (bind _asbp_third_person_character (Utilities|Casting|CastToBP_ThirdPersonCharacter _returnvalue_2)
      (:then
        (Default|ActivateWings _asbp_third_person_character)
        (Default|SetStamina _returnvalue_3 (Variables|Default|GetRequiredStamina))
        (Animation|Montage|PlayMontage (Class|GameplayAbility|GetOwningComponentfromActorInfo) "/Game/Characters/Moth/Anims/v02/DashUp_V2_Montage.DashUp_V2_Montage"
          (:then
            ;[0.15 0.15 0.15 0.5] Fly upward
            (Ability|Tasks|ApplyRootMotionConstantForce "None" (Transformation|GetActorUpVector _returnvalue) 1e+03 1.0 false 0 "MaintainLastRootMotionVelocity" (Transformation|GetVelocity _returnvalue)))
          (:OnCompleted
            (Default|DeactivateWings _asbp_third_person_character :!label _label)
            (Ability|EndAbility))
          (:OnInterrupted
            (goto _label))))
      (:CastFailed
        (Ability|EndAbility :!label _label_2)))
    (else
      (goto _label_2))))

(event Ability|EventOnEndAbility
  (params (bWasCancelled :type Boolean)))