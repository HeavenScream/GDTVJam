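; BP_Shine is a Gameplay Ability that makes the avatar, a moth judging by its montage, shine for a short time.
; After committing, it checks BP_Attributes stamina against RequiredStamina and ends immediately if short.
; Otherwise it passes RequiredStamina to SetStamina, sends the avatar an activate-shine message and plays the shine-on montage.
; A fixed timer then sends the deactivate message and ends the ability.
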(event Custom|FinishedEnergy
  (Class|BPIAbilities|DeactivateShine(Message) (Ability|GetAvatarActorfromActorInfo))
  (Ability|EndAbility))

(event Ability|EventActivateAbility
  (bind _returnvalue (Ability|GetAvatarActorfromActorInfo))
  (bind _returnvalue_2 (Actor|GetComponentbyClass _returnvalue "/Game/ThirdPerson/Blueprints/BP_Attributes.BP_Attributes_C"))
  (Ability|CommitAbility)
  (if (>= (Variables|/Game/ThirdPerson/Blueprints/BP_Attributes.BP_Attributes_C|GetStamina _returnvalue_2) (Variables|Default|GetRequired%20Stamina))
    (Default|SetStamina _returnvalue_2 (Variables|Default|GetRequired%20Stamina))
    (Class|BPIAbilities|ActivateShine(Message) (Ability|GetAvatarActorfromActorInfo))
    (Utilities|Time|SetTimerbyEvent (delegate Custom|FinishedEnergy) 3.0)
    (Animation|Montage|PlayMontage (Class|GameplayAbility|GetOwningComponentfromActorInfo) "/Game/Characters/Moth/Anims/v02/Moth_ShineOn_Montage.Moth_ShineOn_Montage")
    (else
      (Ability|EndAbility))))