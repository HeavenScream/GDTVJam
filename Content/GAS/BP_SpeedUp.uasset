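; Gameplay Ability that gives the third-person character a short, large walk speed boost.
; On activation it saves the avatar's max walk speed, multiplies it and starts a timer.
; When the timer fires, it clears the handle, restores the saved speed and ends the ability.
; The speed is set directly on Character Movement without a Gameplay Effect, and only the timer path restores it.
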(event Custom|Bufftimer
  (Utilities|Time|ClearandInvalidateTimerbyHandle (Variables|Default|GetTimerHandle))
  (Variables|/Script/Engine.CharacterMovementComponent|SetMaxWalkSpeed (Variables|/Script/Engine.Character|GetCharacterMovement (stale Ability|EventActivateAbility _asbp_third_person_character)) (Variables|Default|GetCharacterSpeed))
  (Ability|EndAbility))

(event Ability|EventActivateAbility
  (bind _asbp_third_person_character (Utilities|Casting|CastToBP_ThirdPersonCharacter (Ability|GetAvatarActorfromActorInfo)))
  (Variables|Default|SetCharacterSpeed (Variables|/Script/Engine.CharacterMovementComponent|GetMaxWalkSpeed (Variables|/Script/Engine.Character|GetCharacterMovement _asbp_third_person_character)))
  (Variables|/Script/Engine.CharacterMovementComponent|SetMaxWalkSpeed (Variables|/Script/Engine.Character|GetCharacterMovement _asbp_third_person_character) (* (Variables|Default|GetCharacterSpeed) 1e+01))
  (bind _returnvalue (Utilities|Time|SetTimerbyEvent (delegate Custom|Bufftimer) 1.5))
  (Variables|Default|SetTimerHandle _returnvalue))

(event Ability|EventOnEndAbility
  (params (bWasCancelled :type Boolean)))