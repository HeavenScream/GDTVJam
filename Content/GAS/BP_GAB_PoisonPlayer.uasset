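; Gameplay Ability that poisons its avatar, going by its name the player, with a one-time health hit and visual feedback.
; If the avatar has a BP_Attributes component, it commits, passes a negative value to SetHealth, activates the flicker message and plays the FlyPoisoned montage.
; Montage completion or interruption turns off the flicker message and ends the ability.
; Without that component, nothing runs and EndAbility is never called.
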(event Ability|EventActivateAbility
  (bind _returnvalue (Ability|GetAvatarActorfromActorInfo))
  (bind _returnvalue_2 (Ability|GetAvatarActorfromActorInfo))
  (bind _returnvalue_3 (Actor|GetComponentbyClass _returnvalue "/Game/ThirdPerson/Blueprints/BP_Attributes.BP_Attributes_C"))
  (Utilities|IsValid _returnvalue_3
    (:Is%20Valid
      (Ability|CommitAbility)
      (Default|SetHealth _returnvalue_3 -5.0)
      (Class|BPIAbilities|ActivateFlicker(Message) _returnvalue_2)
      (Animation|Montage|PlayMontage (Class|GameplayAbility|GetOwningComponentfromActorInfo) "/Game/Characters/Moth/Anims/v02/FlyPoisoned_Montage.FlyPoisoned_Montage"
        (:OnCompleted
          _)
        (:OnInterrupted
          _))
      (Class|BPIAbilities|DeactivateFlicker(Message) _returnvalue_2)
      (Ability|EndAbility))))

(event Ability|EventOnEndAbility
  (params (bWasCancelled :type Boolean)))