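; BP_Intoxified is a gameplay ability that applies a damage-over-time intoxication effect to its avatar actor.
; On activation, it checks for a BP_Attributes component on the avatar and starts a looping one-second timer.
; Each tick calls LoseSpirit, which lowers the component's Health by a fixed amount through SetHealth rather than a GameplayEffect.
; Ending the ability clears and invalidates the timer.
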(event Custom|LoseSpirit
  (bind _returnvalue (Ability|GetAvatarActorfromActorInfo))
  (bind _returnvalue_2 (Actor|GetComponentbyClass _returnvalue "/Game/ThirdPerson/Blueprints/BP_Attributes.BP_Attributes_C"))
  (Default|SetHealth _returnvalue_2 (- (Variables|/Game/ThirdPerson/Blueprints/BP_Attributes.BP_Attributes_C|GetHealth _returnvalue_2) 1.0)))

(event Ability|EventActivateAbility
  (Utilities|IsValid (Actor|GetComponentbyClass (Ability|GetAvatarActorfromActorInfo) "/Game/ThirdPerson/Blueprints/BP_Attributes.BP_Attributes_C")
    (:Is%20Valid
      (bind _returnvalue (Utilities|Time|SetTimerbyEvent (delegate Custom|LoseSpirit) 1.0 true))
      (Variables|Default|SetTimerHandle _returnvalue))))

(event Ability|EventOnEndAbility
  (params (bWasCancelled :type Boolean))
  (Utilities|Time|ClearandInvalidateTimerbyHandle (Variables|Default|GetTimerHandle)))